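; BP_CaveDoor is an interactable cave door that opens once when the player character triggers it from nearby.
; Overlap begin and end events set a CharacterNear flag for ThirdPersonCharacter, and the Interact event only proceeds while that flag is set.
; A DoOnce gate then plays the door's Level Sequence through a newly created player, along with a 2D door sound.
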(event Collision|EventActorBeginOverlap
  (params (OtherActor :type Actor%20Object%20Reference))
  ;[1 1 1] Detect presence of character
  (Utilities|Casting|CastToThirdPersonCharacter OtherActor)
  (Variables|Default|SetCharacterNear true))

(event Collision|EventActorEndOverlap
  (params (OtherActor :type Actor%20Object%20Reference))
  ;[1 1 1] Detect presence of character
  (Utilities|Casting|CastToThirdPersonCharacter OtherActor)
  (Variables|Default|SetCharacterNear false))

(event EventInteract
  ;[1 1 1] Open Door
  (if (Variables|Default|GetCharacterNear)
    (Utilities|FlowControl|DoOnce false
      (:Completed
        (bind _returnvalue (Sequencer|Player|CreateLevelSequencePlayer "/Game/Project3/DoorLevelSequence.DoorLevelSequence"))
        (Sequencer|Player|Play _returnvalue :!class /Script/MovieScene.MovieSceneSequencePlayer)
        (Audio|PlaySound2D "/Game/Project3/Audio/Waves/SFX/Folley/A_Cave_Door.A_Cave_Door" 1.0 1.0 0.5 0 0)))))

(fn ConstructionScript)