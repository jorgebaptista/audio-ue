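; BP_Collision_Object is a physics prop that plays layered impact sounds on strong hits.
; Hits above an impulse threshold pick light, medium and heavy stone or wood cues through a GetPhysicalMaterial surface select.
; All three play attached at once, crossfaded by per-layer curves that map normalized impulse to volume.
; A DoOnce reset after a short delay throttles repeated hits.
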(event Collision|EventHit
  (params (MyComp :type Primitive%20Component%20Object%20Reference) (Other :type Actor%20Object%20Reference) (OtherComp :type Primitive%20Component%20Object%20Reference) (bSelfMoved :type Boolean) (HitLocation :type Vector :default "0, 0, 0") (HitNormal :type Vector :default "0, 0, 0") (NormalImpulse :type Vector :default "0, 0, 0") (Hit :type Hit%20Result%20Structure%20%28by%20ref%29))
  (bind _returnvalue (Math|Vector|VectorLength NormalImpulse))
  (bind _surfacetype (Utilities|GetPhysicalMaterial))
  (bind _returnvalue_2 (Math|Float|MapRangeClamped _returnvalue 4e+03 1.25e+05 0.0 1.0))
  (if (>= _returnvalue 1e+04)
    (Utilities|FlowControl|DoOnce false :!label _label
      (:Completed
        (Utilities|PlaySoundCurve (Utilities|Select :Index _surfacetype :SurfaceType_Default "/Game/Project3/Audio/Cues/Collisions/A_Collision_Stone_Light_Cue.A_Collision_Stone_Light_Cue" :SurfaceType1 0 :SurfaceType2 0 :SurfaceType3 "/Game/Project3/Audio/Cues/Collisions/A_Collision_Stone_Light_Cue.A_Collision_Stone_Light_Cue" :SurfaceType4 0 :SurfaceType5 0 :SurfaceType6 "/Game/Project3/Audio/Cues/Collisions/A_Collision_Wood_Light_Cue.A_Collision_Wood_Light_Cue") "/Game/Project3/Audio/Curves/Curve_Collision_Light.Curve_Collision_Light" _returnvalue_2)
        (Utilities|PlaySoundCurve (Utilities|Select :Index _surfacetype :SurfaceType_Default "/Game/Project3/Audio/Cues/Collisions/A_Collision_Stone_Medium_Cue.A_Collision_Stone_Medium_Cue" :SurfaceType1 0 :SurfaceType2 0 :SurfaceType3 "/Game/Project3/Audio/Cues/Collisions/A_Collision_Stone_Medium_Cue.A_Collision_Stone_Medium_Cue" :SurfaceType4 0 :SurfaceType5 0 :SurfaceType6 "/Game/Project3/Audio/Cues/Collisions/A_Collision_Wood_Medium_Cue.A_Collision_Wood_Medium_Cue") "/Game/Project3/Audio/Curves/Curve_Collision_Medium.Curve_Collision_Medium" _returnvalue_2)
        (Utilities|PlaySoundCurve (Utilities|Select :Index _surfacetype :SurfaceType_Default "/Game/Project3/Audio/Cues/Collisions/A_Collision_Stone_Heavy_Cue.A_Collision_Stone_Heavy_Cue" :SurfaceType1 0 :SurfaceType2 0 :SurfaceType3 "/Game/Project3/Audio/Cues/Collisions/A_Collision_Stone_Heavy_Cue.A_Collision_Stone_Heavy_Cue" :SurfaceType4 0 :SurfaceType5 0 :SurfaceType6 "/Game/Project3/Audio/Cues/Collisions/A_Collision_Wood_Heavy_Cue.A_Collision_Wood_Heavy_Cue") "/Game/Project3/Audio/Curves/Curve_Collision_Heavy.Curve_Collision_Heavy" _returnvalue_2)
        (Utilities|FlowControl|Delay 0.15)
        (goto _label Reset)))))

(fn ConstructionScript)