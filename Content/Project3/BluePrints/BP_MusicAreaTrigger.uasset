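; BP_MusicAreaTrigger is a cave trigger actor that switches audio when the player character enters or exits it.
; Begin and end overlap pass a track ID to CheckActorOverlaping, which ignores actors other than player 0.
; It always changes the ambient track on AmbientSoundBp, but changes the MusicBp track only while CanChangeMusic is true.
; On BeginPlay it registers itself with CoinGameStateBP as the MusicAreaTrigger reference.
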(event Collision|EventActorBeginOverlap
  (params (OtherActor :type Actor%20Object%20Reference))
  ;[1 1 1] Entering the Cave Trigger
  (Utilities|CheckActorOverlaping OtherActor 1))

(event EventBeginPlay
  (bind _ascoin_game_state_bp (Utilities|Casting|CastToCoinGameStateBP (Game|GetGameState)))
  (Variables|/Game/Project3/BluePrints/CoinGameStateBP.CoinGameStateBP_C|SetMusicAreaTrigger _ascoin_game_state_bp self))

(event Collision|EventActorEndOverlap
  (params (OtherActor :type Actor%20Object%20Reference))
  ;[1 1 1] Exiting the Cave Trigger
  (Utilities|CheckActorOverlaping OtherActor))

(fn ConstructionScript)