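; BP_Radio is an in-world radio the player operates with number keys while overlapping its collider.
; Overlap events enable and disable input, gating keys for volume, station tuning and power.
; Tuning passes a clamped integer Frequency to the RadioCue audio component as a float parameter.
; Power-off only mutes the cue, so power-on restores the stored volume; volume and tuning keys work only while active.
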(event Collision|EventActorBeginOverlap
  (params (OtherActor :type Actor%20Object%20Reference))
  ;[1 1 1] Overlaping the collider of the Radio
  (if (== OtherActor (Game|GetPlayerCharacter 0))
    (Input|EnableInput (Game|GetPlayerController 0))
    (Variables|Default|SetPlayerColliding true)))

(event Collision|EventActorEndOverlap
  (params (OtherActor :type Actor%20Object%20Reference))
  ;[1 1 1] Overlaping the collider of the Radio
  (if (== (Game|GetPlayerCharacter 0) OtherActor)
    (Input|DisableInput (Game|GetPlayerController 0))
    (Variables|Default|SetPlayerColliding false)))

(event Input|KeyboardEvents|3
  (params (Key :type Key%20Structure))
  ;[1 1 1] Turning Frequency down to change the Radio Station
  (:Pressed
    (if (Variables|Default|GetIsActive)
      (bind _output_get (Variables|Default|SetFrequency (Math|Integer|Max(Integer) (- (Variables|Default|GetFrequency) 1))))
      (Audio|Parameter|SetFloatParameter (Variables|Default|GetRadioCue) "Frequency" (Math|Conversions|ToFloat(Integer) _output_get) :!class /Script/Engine.AudioComponent))))

(event Input|KeyboardEvents|2
  (params (Key :type Key%20Structure))
  (bind _radiocue (Variables|Default|GetRadioCue))
  ;[1 1 1] Turn Volume down
  (:Pressed
    (if (Variables|Default|GetIsActive)
      (bind _output_get (Variables|Default|SetCurrentVolume (Math|Float|Min(Float) (+ (Variables|/Script/Engine.AudioComponent|GetVolumeMultiplier _radiocue) (Variables|Default|GetVolumeAdjust)) 1.0)))
      (Audio|Components|Audio|SetVolumeMultiplier _radiocue _output_get :!class /Script/Engine.AudioComponent))))

(event Input|KeyboardEvents|4
  (params (Key :type Key%20Structure))
  ;[1 1 1] Turning Frequency up to change Radio Station
  (:Pressed
    (if (Variables|Default|GetIsActive)
      (bind _output_get (Variables|Default|SetFrequency (Math|Integer|Min(Integer) (+ (Variables|Default|GetFrequency) 1) 20)))
      (Audio|Parameter|SetFloatParameter (Variables|Default|GetRadioCue) "Frequency" (Math|Conversions|ToFloat(Integer) _output_get) :!class /Script/Engine.AudioComponent))))

(event Input|KeyboardEvents|5
  (params (Key :type Key%20Structure))
  ;[1 1 1] Turning Off
  (:Pressed
    (if (Variables|Default|GetIsActive)
      (Variables|Default|SetIsActive false)
      (Audio|Components|Audio|SetVolumeMultiplier (Variables|Default|GetRadioCue) 0.0 :!class /Script/Engine.AudioComponent))))

(event Input|KeyboardEvents|6
  (params (Key :type Key%20Structure))
  ;[1 1 1] Turning On
  (:Pressed
    (if (not (Variables|Default|GetIsActive))
      (Variables|Default|SetIsActive true)
      (Audio|Components|Audio|SetVolumeMultiplier (Variables|Default|GetRadioCue) (Variables|Default|GetCurrentVolume) :!class /Script/Engine.AudioComponent))))

(event Input|KeyboardEvents|1
  (params (Key :type Key%20Structure))
  (bind _radiocue (Variables|Default|GetRadioCue))
  ;[1 1 1] Turn Volume up
  (:Pressed
    (if (Variables|Default|GetIsActive)
      (bind _output_get (Variables|Default|SetCurrentVolume (Math|Float|Max(Float) (- (Variables|/Script/Engine.AudioComponent|GetVolumeMultiplier _radiocue) (Variables|Default|GetVolumeAdjust)) 0.0)))
      (Audio|Components|Audio|SetVolumeMultiplier _radiocue _output_get :!class /Script/Engine.AudioComponent))))

(fn ConstructionScript)