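; CoinGameStateBP holds the coin game's shared Money and Health values and handles losing.
; AddMoney increases Money, while RemoveHealth subtracts from Health and prints the new value.
; At zero health or below it shows GameOverMenuBP with a loss message, switches to UI-only input with a visible cursor, and pauses the game.
; Otherwise it plays a hurt sound at the player character's location.
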(event Custom|Remove%20Health
  (params (Value :type Integer))
  (bind _returnvalue (Game|GetPlayerController 0))
  (bind _output_get (Variables|Default|SetHealth (- (Variables|Default|GetHealth) Value)))
  (Development|PrintString (Utilities|String|ToString(Integer) _output_get))
  (if (<= _output_get 0)
    (bind _returnvalue_2 (UserInterface|CreateWidget "/Game/Project3/UI/GameOverMenuBP.GameOverMenuBP_C"))
    (Rendering|Components|TextRender|SetText (Variables|/Game/Project3/UI/GameOverMenuBP.GameOverMenuBP_C|GetTextBlock_0 _returnvalue_2) "You loose ! ")
    (Input|SetInputModeUIOnly _returnvalue _returnvalue_2 "DoNotLock")
    (UserInterface|Viewport|AddtoViewport _returnvalue_2 0)
    (Variables|/Script/Engine.PlayerController|SetbShowMouseCursor _returnvalue true)
    (Game|SetGamePaused true)
    (else
      (Audio|PlaySoundatLocation "/Game/Project3/Audio/Cues/Hurt_Cue.Hurt_Cue" (Transformation|GetActorLocation (Game|GetPlayerCharacter 0)) "0, 0, 0" 1.0 1.0 0.0 0 0 0))))

(event Custom|AddMoney
  (params (NewParam :type Integer))
  (Variables|Default|SetMoney (+ NewParam (Variables|Default|GetMoney))))

(fn ConstructionScript)