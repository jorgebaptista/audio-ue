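; A fire hazard actor that cycles on and off, draining health from a nearby player while it burns.
; BeginPlay runs an endless delay loop that toggles the particle system and a repeating damage timer, replaying audio on each ignition.
; Overlap events track whether a ThirdPersonCharacter is nearby, and each timer tick then removes health through CoinGameStateBP.
; The damage timer first starts after one full off phase.
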(event Custom|Remove%20Health
  ;[1 1 1] Damage
  (if (Variables|Default|GetCharacter%20Nearby)
    (bind _ascoin_game_state_bp (Utilities|Casting|CastToCoinGameStateBP (Game|GetGameState)))
    (Default|RemoveHealth _ascoin_game_state_bp 20)))

(event EventBeginPlay
  (bind _particlesystem (Variables|Default|GetParticlesystem))
  ;[1 1 1] on and off
  (Utilities|FlowControl|Delay 4.0 :!label _label)
  (Components|Activation|Deactivate _particlesystem)
  (Utilities|Time|ClearTimerbyFunctionName 0 "Remove Health")
  (Utilities|FlowControl|Delay 4.0)
  (Utilities|Time|SetTimerbyFunctionName 0 "Remove Health" 1.0 true)
  (Components|Activation|Activate _particlesystem false)
  (Audio|Components|Audio|Play (Variables|Default|GetAudioComponent) 0.0)
  (goto _label))

(event Collision|EventActorBeginOverlap
  (params (OtherActor :type Actor%20Object%20Reference))
  ;[1 1 1] detect presence
  (Utilities|Casting|CastToThirdPersonCharacter OtherActor)
  (Variables|Default|SetCharacter%20Nearby true))

(event Collision|EventActorEndOverlap
  (params (OtherActor :type Actor%20Object%20Reference))
  ;[1 1 1] detect presence
  (Utilities|Casting|CastToThirdPersonCharacter OtherActor)
  (Variables|Default|SetCharacter%20Nearby false))

(fn ConstructionScript)