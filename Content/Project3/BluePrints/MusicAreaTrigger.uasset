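; Trigger actor that switches the music and ambient sound when the player enters or leaves an area, which its comments identify as a cave.
; Begin and end overlap events both call CheckActorOverlaping with a track ID, one for inside and one for outside.
; That function ignores any actor other than player character 0, then passes the ID to MusicBp and AmbientSoundBp to change their tracks.
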(event Collision|EventActorBeginOverlap
  (params (OtherActor :type Actor%20Object%20Reference))
  ;[1 1 1] Entering the Cave Trigger
  (Utilities|CheckActorOverlaping OtherActor 1))

(event Collision|EventActorEndOverlap
  (params (OtherActor :type Actor%20Object%20Reference))
  ;[1 1 1] Exiting the Cave Trigger
  (Utilities|CheckActorOverlaping OtherActor))

(fn ConstructionScript)