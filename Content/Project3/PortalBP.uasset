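; Portal actor that acts as the level exit, ending the game once the player has collected enough money.
; On BeginPlay it caches the CoinGameStateBP, then checks its Money when a ThirdPersonCharacter overlaps the Capsule.
; An exact match with the hardcoded target shows GameOverMenuBP with UI-only input and a cursor, then pauses the game.
; Otherwise the portal mesh briefly flashes red through a timed material swap.
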(event OnComponentBeginOverlap(Capsule)
  (params (OverlappedComponent :type Primitive%20Component%20Object%20Reference) (OtherActor :type Actor%20Object%20Reference) (OtherComp :type Primitive%20Component%20Object%20Reference) (OtherBodyIndex :type Integer) (bFromSweep :type Boolean) (SweepResult :type Hit%20Result%20Structure%20%28by%20ref%29))
  (bind _returnvalue (Game|GetPlayerController 0))
  ;[1 1 1] Check win
  (Utilities|Casting|CastToThirdPersonCharacter OtherActor)
  (if (== (Variables|/Game/Project3/CoinGameStateBP.CoinGameStateBP_C|GetMoney (Variables|Default|GetGameState)) 2)
    (bind _returnvalue_2 (UserInterface|CreateWidget "/Game/Project3/GameOverMenuBP.GameOverMenuBP_C"))
    (Input|SetInputModeUIOnly _returnvalue _returnvalue_2 "DoNotLock")
    (UserInterface|Viewport|AddtoViewport _returnvalue_2 0)
    (Variables|/Script/Engine.PlayerController|SetbShowMouseCursor _returnvalue true)
    (Game|SetGamePaused true)
    (else
      (CallFunction|FlashRed))))

(event Custom|Flash%20Red
  (bind _staticmesh (Variables|Default|GetStaticMesh))
  ;[1 1 1] flash red
  (Rendering|Material|SetMaterial _staticmesh 0 "/Game/Material/LaserMat_Inst3.LaserMat_Inst3")
  (Utilities|FlowControl|Delay 0.5)
  (Rendering|Material|SetMaterial _staticmesh 0 "/Game/Material/LaserMat_Inst2.LaserMat_Inst2"))

(event EventBeginPlay
  ;[1 1 1] Get game state
  (bind _ascoin_game_state_bp (Utilities|Casting|CastToCoinGameStateBP (Game|GetGameState)))
  (Variables|Default|SetGameState _ascoin_game_state_bp))

(fn ConstructionScript)